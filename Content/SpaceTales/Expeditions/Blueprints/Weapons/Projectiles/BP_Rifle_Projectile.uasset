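; BP_Rifle_Projectile is a rifle bullet projectile Blueprint with a collision sphere and a projectile movement component.
; Its graph holds only debug output: BeginPlay briefly prints the movement component's max speed, and a sphere hit prints the hit time plus two colored default messages.
; Overlap and Tick are empty, the construction script just calls its parent, and the graph applies no damage or impact effects.
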(event OnComponentHit(BulletCollisionSphere)
  (params (HitComponent :type Primitive%20Component%20Object%20Reference) (OtherActor :type Actor%20Object%20Reference) (OtherComp :type Primitive%20Component%20Object%20Reference) (NormalImpulse :type Vector :default "0, 0, 0") (Hit :type Hit%20Result%20Structure%20%28by%20ref%29))
  (Development|PrintString (Utilities|String|ToString(Float) (.Time (Collision|BreakHitResult Hit))) true true "(R=0.112119,G=1.000000,B=0.000000,A=1.000000)")
  (Development|PrintString "Hello" true true "(R=1.000000,G=0.000000,B=0.025124,A=1.000000)")
  (Development|PrintString "Hello" true true "(R=1.000000,G=0.907705,B=0.000000,A=1.000000)"))

(event EventBeginPlay
  (Development|PrintString (Utilities|String|ToString(Float) (Class|MovementComponent|GetMaxSpeed (Variables|Default|GetBulletProjectileMovement))) true true "(R=0.000000,G=0.660000,B=1.000000,A=1.000000)" 0.001))

(event Collision|EventActorBeginOverlap
  (params (OtherActor :type Actor%20Object%20Reference)))

(event EventTick
  (params (DeltaSeconds :type Float%20%28single-precision%29)))

(fn ConstructionScript
  (|CallParentFunction))