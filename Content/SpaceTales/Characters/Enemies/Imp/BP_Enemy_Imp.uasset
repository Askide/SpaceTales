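; Imp enemy Blueprint that extends a parent enemy class with a fixed walk speed and custom attack and stun rules.
; Stuns have a 22% chance to set GotAgression and lengthen the stun time range before the parent logic runs.
; That flag blocks attacks until the stun timer clears it, though the added time is never reverted, so it accumulates.
; Attacks also wait until no montage is playing.
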(event EventBeginPlay
  (|CallParentFunction)
  (Variables|/Script/Engine.CharacterMovementComponent|SetMaxWalkSpeed (Variables|Character|GetCharacterMovement) 3e+02))

(event Collision|EventActorBeginOverlap
  (params (OtherActor :type Actor%20Object%20Reference)))

(event EventTick
  (params (DeltaSeconds :type Float%20%28single-precision%29))
  (|CallParentFunction DeltaSeconds))

(event EventAttack
  (if (and (not (Variables|Default|GetbGotAgression)) (not (Utilities|IsValid (Animation|GetCurrentMontage :!class /Script/Engine.Character))))
    (|CallParentFunction)))

(fn ConstructionScript
  (|CallParentFunction))

(fn StunEnable
  (if (Math|Random|RandomBoolwithWeight 0.22)
    (Variables|Default|SetbGotAgression true)
    (Variables|Default|SetStunTimeMin (+ (Variables|Default|GetStunTimeMin) 3.0))
    (Variables|Default|SetStunTimeMax (+ (Variables|Default|GetStunTimeMax) 3.0)))
  (|CallParentFunction)
  (return))

(fn StunTimerEnd
  (Variables|Default|SetbGotAgression false)
  (|CallParentFunction))