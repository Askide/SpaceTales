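; Enemy character Blueprint for the Vodyanoy, extending a parent enemy class that supplies the distance-to-player value and the base attack.
; Each tick it maps player distance to max walk speed, slowing the enemy as it closes in on the player.
; On attack, it snaps the AI controller's control rotation toward the player before running the parent attack logic.
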(event EventBeginPlay)

(event Collision|EventActorBeginOverlap
  (params (OtherActor :type Actor%20Object%20Reference)))

(event EventTick
  (params (DeltaSeconds :type Float%20%28single-precision%29))
  (|CallParentFunction DeltaSeconds)
  (Variables|/Script/Engine.CharacterMovementComponent|SetMaxWalkSpeed (Variables|Character|GetCharacterMovement) (Math|Float|MapRangeClamped (Variables|Default|GetCurrentDistanceToPlayer) 6e+02 8e+02 2e+02 4e+02)))

(event EventAttack
  (Pawn|SetControlRotation (AI|GetAIController self) (Math|Rotator|FindLookatRotation (Transformation|GetActorLocation) (Transformation|GetActorLocation (Game|GetPlayerCharacter 0))))
  (|CallParentFunction))

(fn ConstructionScript
  (|CallParentFunction))