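; BP_MainCharacter is the main character Blueprint, handling weapon switching, firing and item pickup.
; Number keys equip pistol or rifle from BackpackWeapons with montages, the pistol as its montage starts and the rifle on completion.
; Fire input toggles the current weapon's fire state, while reload, attack and death events play supplied montages.
; Capsule overlaps pass InventoryComponent through BPI_PickupItems, and Tick prints ammo counts for debugging.
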(event OnComponentBeginOverlap(CapsuleComponent)
  (params (OverlappedComponent :type Primitive%20Component%20Object%20Reference) (OtherActor :type Actor%20Object%20Reference) (OtherComp :type Primitive%20Component%20Object%20Reference) (OtherBodyIndex :type Integer) (bFromSweep :type Boolean) (SweepResult :type Hit%20Result%20Structure%20%28by%20ref%29))
  (if (Utilities|DoesObjectImplementInterface OtherActor "/Game/SpaceTales/Expeditions/Interfaces/BPI_PickupItems.BPI_PickupItems_C")
    (Class|BPIPickupItems|TrytoPickUp(Message) OtherActor (Variables|Default|GetInventoryComponent))))

(event EventTick
  (params (DeltaSeconds :type Float%20%28single-precision%29))
  (|CallParentFunction DeltaSeconds)
  (Utilities|FlowControl|Sequence
    (:then_0
      (for _array_element (Variables|/Script/ST.InventoryComponent|GetAmmoSlots (Variables|Default|GetInventoryComponent))
        (Development|PrintString (Utilities|String|ToString(Integer) (.Count (Utilities|Struct|BreakAmmoSlot _array_element))) true true "(R=1.000000,G=0.942050,B=0.140625,A=1.000000)" 0.001)))
    (:then_1
      (Development|PrintString (Utilities|String|ToString(Integer) (Class|STWeaponDefault|GetWeaponRound (Variables|Default|GetCurrentWeapon))) true true "(R=0.000000,G=1.000000,B=0.823006,A=1.000000)" 0.001))))

(event EventCharAttackBP
  (params (CharAnim :type Anim%20Montage%20Object%20Reference))
  (Animation|Montage|PlayMontage (Variables|Character|GetMesh) CharAnim))

(event EventBeginPlay
  (|CallParentFunction))

(event EventCharDeadBP
  (params (CharAnim :type Anim%20Montage%20Object%20Reference))
  (Animation|Montage|PlayMontage (Variables|Character|GetMesh) CharAnim))

(event EventWeaponReloadStartBP
  (params (CharAnim :type Anim%20Montage%20Object%20Reference))
  (Animation|Montage|PlayMontage (Variables|Character|GetMesh) CharAnim))

(event Input|ActionEvents|InputActionFire
  (params (Key :type Key%20Structure :default "None"))
  (bind _currentweapon (Variables|Default|GetCurrentWeapon))
  (:Pressed
    (Utilities|IsValid _currentweapon
      (:Is%20Valid
        (Class|STWeaponDefault|SetWeaponStateFire _currentweapon true))))
  (:Released
    (Utilities|IsValid _currentweapon
      (:Is%20Valid
        (Class|STWeaponDefault|SetWeaponStateFire _currentweapon false)))))

(event Input|KeyboardEvents|1
  (params (Key :type Key%20Structure :default "None"))
  (:Pressed
    (Animation|Montage|PlayMontage (Variables|Character|GetMesh) "/Game/SpaceTales/Characters/MainCharacter/Animations/Actions/Equip_Pistol_Standing_Anim_Montage.Equip_Pistol_Standing_Anim_Montage"
      (:then
        (Class|STCharacter|EquipNewWeapon (Utilities|Array|Get(acopy) (Variables|Default|GetBackpackWeapons)))))))

(event Input|KeyboardEvents|2
  (params (Key :type Key%20Structure :default "None"))
  (:Pressed
    (Animation|Montage|PlayMontage (Variables|Character|GetMesh) "/Game/SpaceTales/Characters/MainCharacter/Animations/Actions/Equip_Rifle_Standing_Anim_Montage.Equip_Rifle_Standing_Anim_Montage"
      (:OnCompleted
        (Class|STCharacter|EquipNewWeapon (Utilities|Array|Get(acopy) (Variables|Default|GetBackpackWeapons) 1))))))

(fn ConstructionScript)